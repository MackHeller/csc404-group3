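; Hook actor that lives three seconds and sticks to what it hits, likely a fired grappling or projectile hook.
; On hit it attaches to the other actor at its current world transform and disables its capsule collision, unless that actor is another Hook.
; Non-player hits spawn short-lived particles and a sound: electricity for one force field matched by hardcoded object name, sparks and metal clink otherwise.
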(event `self.ReceiveBeginPlay`
  (`self.SetLifeSpan` 3.0))

(event `self.ReceiveHit`
  (params (MyComp :type "PrimitiveComponent Object Reference") (Other :type "Actor Object Reference") (OtherComp :type "PrimitiveComponent Object Reference") (bSelfMoved :type Boolean) (HitLocation :type "Vector Structure") (HitNormal :type "Vector Structure") (NormalImpulse :type "Vector Structure") (Hit :type "HitResult Structure (by ref)"))
  (bind _returnvalue (`self.K2_GetActorLocation`))
  (bind _returnvalue_2 (`self.K2_GetActorLocation`))
  (bind _returnvalue_3 (`KismetStringLibrary.EqualEqual_StrStr` (`KismetSystemLibrary.GetObjectName` Other) "Forcefield_Collision_01_2"))
  (`|ExecutionSequence`
    (:`then_0`
      (if (!= (`GameplayStatics.GetObjectClass` Other) "Hook_C")
        (`self.K2_AttachToActor` Other "None" "KeepWorld" "KeepWorld" "KeepWorld")
        (`PrimitiveComponent.SetCollisionEnabled` (`self.CollisionCapsule`) "NoCollision")))
    (:`then_2`
      ;[1 1 1] spawn sparks for hitting env objects
      (if (== (`GameplayStatics.GetObjectClass` Other) "/Game/Blueprints/Player.Player_C")
        _
        (elif _returnvalue_3
          ;[1 1 1] Spawn electricity and sparks for hiting force field and sound
          (if _returnvalue_3
            (`|ExecutionSequence`
              (:`then_0`
                (bind _returnvalue_4 (`GameplayStatics.SpawnEmitterAtLocation` "/Game/Art/Particles/gh_electricty_01_p.gh_electricty_01_p" _returnvalue))
                (`KismetSystemLibrary.Delay` 0.9)
                (`ActorComponent.K2_DestroyComponent` _returnvalue_4))
              (:`then_1`
                (`GameplayStatics.SpawnSoundAtLocation` "/Game/Art/Sound/electric_zap.electric_zap" _returnvalue))))
          (else
            (`|ExecutionSequence`
              (:`then_0`
                (bind _returnvalue_5 (`GameplayStatics.SpawnEmitterAtLocation` "/Game/Art/Particles/Sparks_red.Sparks_red" _returnvalue_2))
                (`KismetSystemLibrary.Delay` 0.5)
                (`ActorComponent.K2_DestroyComponent` _returnvalue_5))
              (:`then_1`
                ;[1 1 1] sound for hitting env object
                (`GameplayStatics.SpawnSoundAtLocation` "/Game/Art/Sound/gh_metal_ting.gh_metal_ting" _returnvalue_2)))))))))

(fn `UserConstructionScript`)