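; BowCaster weapon Blueprint that fires Bolt actors with a short recharge between shots.
; Tick accumulates a clamped recharge timer and sets CanFire once it passes the threshold of just under a second.
; FireBow checks that flag, calls Fire, resets the recharge and plays a laser sound at the actor's location.
; Fire spawns the bolt at the Arrow component's position plus a rotated offset, aligned to the arrow's rotation.
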(event `self.ReceiveTick`
  (params (DeltaSeconds :type "Float (single-precision)"))
  ;[1 1 1] update bowcaster bolt recharge
  (`|ExecutionSequence`
    (:`then_0`
      (set `self.recharge` (`KismetMathLibrary.FClamp` (+ (`self.recharge`) DeltaSeconds) 0.0 0.81)))
    (:`then_1`
      (if (> (`self.recharge`) 0.8)
        (set `self.CanFire` true)))))

(event `FireBow`
  (if (`self.CanFire`)
    (set `self.CanFire` false)
    (`self.Fire`)
    (set `self.recharge` 0.0)
    (`GameplayStatics.SpawnSoundAtLocation` "/Game/Art/Sound/321101__nsstudios__laser2.321101__nsstudios__laser2" (`self.K2_GetActorLocation`))))

(fn `Fire`
  (bind _arrow (`self.Arrow`))
  (bind _returnvalue (`SceneComponent.K2_GetComponentRotation` _arrow))
  (`|SpawnActorFromClass` "/Game/Blueprints/Bolt.Bolt_C" (`KismetMathLibrary.MakeTransform` (+ (`SceneComponent.K2_GetComponentLocation` _arrow) (`KismetMathLibrary.GreaterGreater_VectorRotator` (`self.Offset`) _returnvalue)) _returnvalue) "Undefined" "OverrideRootScale" null null)
  (return))

(fn `UserConstructionScript`)