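; Game mode for BowCaster's four-player rounds, running the main menu, round countdown, kill scores and respawns.
; Tick polls each player's health; deaths of the first three credit every other player, while the fourth player's death only resets them.
; A Delay in Tick drives the timer, which at zero saves last-round scores, shows EndGame, resets and pauses.
; ResetPlayer teleports randomly, inflates health for three seconds, then teleports again and restores health.
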(event `self.ReceiveTick`
  (params (DeltaSeconds :type "Float (single-precision)"))
  (bind _returnvalue (`GameplayStatics.GetPlayerCharacter` 3))
  (bind _returnvalue_2 (`GameplayStatics.GetPlayerCharacter` 0))
  (bind _returnvalue_3 (`GameplayStatics.GetPlayerCharacter` 1))
  (bind _returnvalue_4 (`GameplayStatics.GetPlayerCharacter` 2))
  (`|ExecutionSequence`
    (:`then_0`
      ;[1 1 1] Determine if a player died
      (`|ExecutionSequence`
        (:`then_0`
          (bind _asplayer (cast `/Game/Blueprints/Player` _returnvalue_2))
          (if (<= (`/Game/Blueprints/Player.Health` _asplayer) 0)
            (bind _asplayer_2 (cast `/Game/Blueprints/Player` _returnvalue_2))
            (`self.ResetPlayer` _asplayer_2)
            ;[1 1 1] Kills Score Update
            (bind _result (`/Engine/EditorBlueprintResources/StandardMacros.IncrementInt` (`self.p2kills`))
              (:`  `
                (set `self.p2kills` _result)
                (bind _result_2 (`/Engine/EditorBlueprintResources/StandardMacros.IncrementInt` (`self.p3kills`))
                  (:`  `
                    (set `self.p3kills` _result_2)
                    (bind _result_3 (`/Engine/EditorBlueprintResources/StandardMacros.IncrementInt` (`self.p4kills`))
                      (:`  `
                        (set `self.p4kills` _result_3)))))))))
        (:`then_1`
          (bind _asplayer_3 (cast `/Game/Blueprints/Player` _returnvalue_3))
          (if (<= (`/Game/Blueprints/Player.Health` _asplayer_3) 0)
            (bind _asplayer_4 (cast `/Game/Blueprints/Player` _returnvalue_3))
            (`self.ResetPlayer` _asplayer_4)
            (bind _result_4 (`/Engine/EditorBlueprintResources/StandardMacros.IncrementInt` (`self.p1kills`))
              (:`  `
                (set `self.p1kills` _result_4)
                (bind _result_5 (`/Engine/EditorBlueprintResources/StandardMacros.IncrementInt` (`self.p3kills`))
                  (:`  `
                    (set `self.p3kills` _result_5)
                    (bind _result_6 (`/Engine/EditorBlueprintResources/StandardMacros.IncrementInt` (`self.p4kills`))
                      (:`  `
                        (set `self.p4kills` _result_6)))))))))
        (:`then_2`
          (bind _asplayer_5 (cast `/Game/Blueprints/Player` _returnvalue_4))
          (if (<= (`/Game/Blueprints/Player.Health` _asplayer_5) 0)
            (bind _asplayer_6 (cast `/Game/Blueprints/Player` _returnvalue_4))
            (`self.ResetPlayer` _asplayer_6)
            (bind _result_7 (`/Engine/EditorBlueprintResources/StandardMacros.IncrementInt` (`self.p1kills`))
              (:`  `
                (set `self.p1kills` _result_7)
                (bind _result_8 (`/Engine/EditorBlueprintResources/StandardMacros.IncrementInt` (`self.p2kills`))
                  (:`  `
                    (set `self.p2kills` _result_8)
                    (bind _result_9 (`/Engine/EditorBlueprintResources/StandardMacros.IncrementInt` (`self.p4kills`))
                      (:`  `
                        (set `self.p4kills` _result_9)))))))))
        (:`then_3`
          (bind _asplayer_7 (cast `/Game/Blueprints/Player` _returnvalue))
          (if (<= (`/Game/Blueprints/Player.Health` _asplayer_7) 0)
            (bind _asplayer_8 (cast `/Game/Blueprints/Player` _returnvalue))
            (`self.ResetPlayer` _asplayer_8)))))
    (:`then_1`
      ;[1 1 1] Timer
      (`KismetSystemLibrary.Delay` 1.0)
      (set `self.seconds` (- (`self.seconds`) 1))
      (if (< (`self.seconds`) 0)
        (set `self.minutes` (- (`self.minutes`) 1))
        (set `self.seconds` 59))
      (if (== (`self.seconds`) 0)
        (if (== (`self.minutes`) 0)
          ;[1 1 1] End Game Logic
          (bind _returnvalue_5 (`|CreateWidget` "/Game/Blueprints/EndGame.EndGame_C"))
          (set `self.lastRoundP1Kills` (`self.p1kills`))
          (set `self.lastRoundP2Kills` (`self.p2kills`))
          (set `self.lastRoundP3Kills` (`self.p3kills`))
          (set `self.lastRoundP4Kills` (`self.p4kills`))
          (`UserWidget.AddToViewport` _returnvalue_5 0)
          (set `self.seconds` (`self.defaultSeconds`))
          (set `self.minutes` (`self.defaultMinutes`))
          (set `self.p1kills` 0)
          (set `self.p2kills` 0)
          (set `self.p3kills` 0)
          (set `self.p4kills` 0)
          (bind _asplayer_9 (cast `/Game/Blueprints/Player` (`GameplayStatics.GetPlayerCharacter` 0)))
          (`self.ResetPlayer` _asplayer_9)
          (bind _asplayer_10 (cast `/Game/Blueprints/Player` (`GameplayStatics.GetPlayerCharacter` 1)))
          (`self.ResetPlayer` _asplayer_10)
          (bind _asplayer_11 (cast `/Game/Blueprints/Player` (`GameplayStatics.GetPlayerCharacter` 2)))
          (`self.ResetPlayer` _asplayer_11)
          (bind _asplayer_12 (cast `/Game/Blueprints/Player` (`GameplayStatics.GetPlayerCharacter` 3)))
          (`self.ResetPlayer` _asplayer_12)
          (`GameplayStatics.SetGamePaused` true))))))

(event `self.ReceiveBeginPlay`
  (`|ExecutionSequence`
    (:`then_0`
      ;[1 1 1] Show Main Menu
      (bind _returnvalue (`|CreateWidget` "/Game/Blueprints/MainMenu.MainMenu_C"))
      (`UserWidget.AddToViewport` _returnvalue 0)
      (`GameplayStatics.SetGamePaused` true))
    (:`then_1`
      ;[1 1 1] Set round timer defaults
      (set `self.defaultSeconds` 3)
      (set `self.defaultMinutes` 0)
      (set `self.seconds` (`self.defaultSeconds`))
      (set `self.minutes` (`self.defaultMinutes`)))))

(event `ResetPlayer`
  (params (`Player Character` :type "/Game/Blueprints/Player Object Reference"))
  (bind _returnvalue (`KismetMathLibrary.RandomPointInBoundingBox` (`KismetMathLibrary.MakeVector` 69.0 8.0 211.0) (`KismetMathLibrary.MakeVector` 3000.0 1000.0 1000.0)))
  ;[1 1 1] Reset the player
  (`|ExecutionSequence`
    (:`then_0`
      ;;[1 1 1] Temporary patch to teleport player out of map while the death screen shows
      (`self.K2_TeleportTo` :`self` `Player Character` :`DestLocation` _returnvalue)
      (set `/Game/Blueprints/Player.Health` 99999 `Player Character`)
      (`KismetSystemLibrary.Delay` 3.0)
      (`self.K2_TeleportTo` :`self` `Player Character` :`DestLocation` _returnvalue)
      (set `/Game/Blueprints/Player.Health` 100 `Player Character`)
      (`/Game/Blueprints/Player.StopMoving` `Player Character`))))

(fn `UserConstructionScript`)