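; Player character for a bow-caster shooter with free-rotation look, switchable cameras, health, bolt knockback and last-hit tracking.
; Movement launches the capsule along the camera's forward vector until a hit stops it.
; A traced harpoon animates a Cable to the hit point, and the grapple input applies force toward it.
; Tick aims the BowCaster child actor and attempts idle damage, though the AsPlayer reference it checks is never set.
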(event OnComponentHit(CapsuleComponent)
  (params (HitComponent :type Primitive%20Component%20Object%20Reference) (OtherActor :type Actor%20Object%20Reference) (OtherComp :type Primitive%20Component%20Object%20Reference) (NormalImpulse :type Vector :default "0, 0, 0") (Hit :type Hit%20Result%20Structure%20%28by%20ref%29))
  ;[1 1 1] Player movement
  (if (or (Variables|Default|GetMoving) (Variables|Default|GetGrappling))
    (Variables|Default|SetMoving false)
    (Variables|Default|SetGrappling false)
    (Variables|Default|SetCanPickDirection true)
    (CallFunction|StopMoving)
    (bind _asplayer_controller (Utilities|Casting|CastToPlayerController (Pawn|GetController)))
    (Game|Feedback|PlayDynamicForceFeedback _asplayer_controller 0.1 0.1 true true true true)))

(event Custom|TakeDamage
  (params (damage :type Integer))
  ;[1 1 1] Taking Damage
  (bind _output_get (Variables|Default|SetHealth (- (Variables|Default|GetHealth) damage)))
  (if (<= _output_get 0)
    (Variables|Default|SetHealth 0)
    (bind _asplayer_controller (Utilities|Casting|CastToPlayerController (Pawn|GetController)))
    (bind _returnvalue (UserInterface|CreateWidget "/Game/HUD/YouDied.YouDied_C" _asplayer_controller))
    (UserInterface|Viewport|AddtoPlayerScreen _returnvalue)
    (Game|Feedback|PlayDynamicForceFeedback _asplayer_controller 1.0 1.0 true true true true)))

(event Custom|BugFoundKillPlayer
  ;[1 1 1] Bug Found, Show message and kill player
  (bind _asplayer_controller (Utilities|Casting|CastToPlayerController (Pawn|GetController)))
  (bind _returnvalue (UserInterface|CreateWidget "/Game/HUD/EasterEgg.EasterEgg_C" _asplayer_controller))
  (UserInterface|Viewport|AddtoPlayerScreen _returnvalue)
  (Utilities|FlowControl|Delay 3.5)
  (CallFunction|TakeDamage 99999999))

(event Custom|StopGrapple
  (bind _cable (Variables|Default|GetCable))
  ;[1 1 1] Harpoon/Change View
  ;;[1 1 1] Stop Grapple and reset cable length
  (Variables|Default|SetHooked false)
  (Transformation|SetWorldLocation (Variables|Default|GetCable) (Transformation|GetActorLocation) false false)
  (bind _output_get (Variables|/Script/CableComponent.CableComponent|SetCableLength _cable 0.0))
  (Variables|Default|SetNewCableLength _output_get)
  (Variables|/Script/CableComponent.CableComponent|SetEndLocation _cable "20.000000, 0,0.000000")
  (Variables|Default|SetHook%20Location "20.000000, 0, 0"))

(event Custom|StopMoving
  (bind _charactermovement (Variables|Character|GetCharacterMovement))
  (bind _updatedprimitive (Variables|/Script/Engine.MovementComponent|GetUpdatedPrimitive _charactermovement))
  ;[1 1 1] Player movement
  (Utilities|FlowControl|Sequence
    (:then_0
      (Class|PrimitiveComponent|SetAllPhysicsLinearVelocity _updatedprimitive "0, 0, 0" false)
      (Components|Movement|StopMovementImmediately (Variables|Character|GetCharacterMovement)))
    (:then_1
      (Class|PrimitiveComponent|SetAllPhysicsAngularVelocity _updatedprimitive (Math|Vector|RotateVector "0, 0, 0" "0, 0, 0") false)
      (Class|NavMovementComponent|StopActiveMovement (Variables|Character|GetCharacterMovement)))))

(event Custom|setBowRoation
  ;[1 1 1] Set Bow Rotation
  (Transformation|SetWorldRotation (Variables|Default|GetBowCaster) (|RoundRotation (Transformation|GetWorldRotation (Variables|Default|GetCamera))) false false))

(event Custom|GrappleWhenPressG
  ;[1 1 1] Harpoon/Change View
  ;;[1 1 1] Grapple when press G
  (if (Variables|Default|GetGIsPressed)
    (CallFunction|GrapplingMove)
    (Variables|/Script/CableComponent.CableComponent|SetCableLength (Variables|Default|GetCable) (Math|Vector|VectorLength (- (Transformation|GetActorLocation) (Variables|Default|GetHook%20Location))))
    (CallFunction|StopGrapple)))

(event Custom|Grappling%20Move
  ;[1 1 1] Harpoon/Change View
  ;;[1 1 1] Grappling Move
  (Variables|Default|SetGrappling true)
  (Physics|AddForce (Variables|/Script/Engine.MovementComponent|GetUpdatedPrimitive (Variables|Character|GetCharacterMovement)) (* (- (Variables|Default|GetHook%20Location) (Transformation|GetActorLocation)) 5e+01) "None" true))

(event EventBeginPlay
  (bind _cable (Variables|Default|GetCable))
  (Utilities|FlowControl|Sequence
    (:then_1
      ;[1 1 1] Spawn Player
      (Utilities|Casting|CastToBowCasterGameMode (Game|GetGameMode))
      (Variables|Default|SetSpawn%20Transform (Transformation|GetActorTransform)))
    (:then_2
      ;[1 1 1] Harpoon/Change View
      ;;[1 1 1] Set cable parameters
      (Rendering|SetVisibility _cable false false)
      (Variables|/Script/CableComponent.CableComponent|SetCableLength _cable 0.0)
      (Variables|/Script/CableComponent.CableComponent|SetCableWidth _cable 2.0)
      (Variables|/Script/CableComponent.CableComponent|SetEndLocation _cable "20.000000,0.000000,0.000000")
      (Variables|Default|SetHook%20Location "20.000000, 0, 0"))
    (:then_3
      (Variables|Default|SetHealth 120))
    (:then_4
      (Components|Movement|StopMovementImmediately (Variables|Character|GetCharacterMovement)))
    (:then_5
      ;[1 1 1] SetOwnerOfBowCaster
      (bind _asbow_caster (Utilities|Casting|CastToBowCaster (Variables|/Script/Engine.ChildActorComponent|GetChildActor (Variables|Default|GetBowCaster))))
      (Variables|/Game/Blueprints/BowCaster.BowCaster_C|SetShooter _asbow_caster (Variables|Default|GetPlayerID))
      (Variables|Default|SetLastHit 10))))

(event EventTick
  (params (DeltaSeconds :type Float%20%28single-precision%29))
  (bind _cable (Variables|Default|GetCable))
  (bind _bowcaster (Variables|Default|GetBowCaster))
  (bind _returnvalue (Transformation|GetWorldLocation _bowcaster))
  (Utilities|FlowControl|Sequence
    (:then_0
      ;[1 1 1] Player movement
      (CallFunction|SetBowRoation)
      (if (and (Variables|Default|GetMoving) (Variables|Default|GetCanPickDirection))
        (Variables|Default|SetCanPickDirection false)
        (Physics|AddForce (Variables|/Script/Engine.MovementComponent|GetUpdatedPrimitive (Variables|Character|GetCharacterMovement)) (* (Math|Vector|GetForwardVector (Variables|Default|GetCamera)) 5.8e+04) "None" true)))
    (:then_1
      ;[1 1 1] Player takes damage if not moving
      (bind _ispaused (CallFunction|IsGamePaused))
      (if (not _ispaused)
        (Utilities|FlowControl|Delay 1.0)
        (if (Math|Vector|Equal(Vector) (Transformation|GetVelocity (stale _asplayer)) "0, 0, 0" 0.001)
          (CallFunction|TakeDamage 2))))
    (:then_2
      ;[1 1 1] laser tracer
      (bind _outactors (Actor|GetAllActorsOfClass "/Game/Blueprints/Bolt.Bolt_C"))
      (Collision|LineTraceByChannel _returnvalue (+ (* (Math|Vector|GetForwardVector (Transformation|GetWorldRotation _bowcaster)) 1.5e+03) _returnvalue) "TraceTypeQuery1" false _outactors "ForOneFrame"))
    (:then_3
      ;[1 1 1] Harpoon/Change View
      (if (and (Variables|Default|GetHooked) (not (Variables|Default|GetGrappling)))
        (CallFunction|GrapplewhenPressG)
        (if (Variables|Default|GetHook%20Move%20Finished)
          (Utilities|FlowControl|Sequence
            (:then_0
              ;;[1 1 1] Move Start position of the cable
              (Transformation|SetWorldLocationAndRotation (Variables|Default|GetCable) (Math|Interpolation|VInterpTo (Transformation|GetWorldLocation (Variables|Default|GetCable)) (Variables|Default|GetHook%20Location) (Utilities|Time|GetWorldDeltaSeconds) 2.5e+02) (Math|Rotator|FindLookatRotation (Transformation|GetActorLocation) (Variables|Default|GetHook%20Location)) false false)
              ;;[1 1 1] Set cable length
              (bind _output_get (Variables|/Script/CableComponent.CableComponent|SetCableLength _cable (+ (Math|Vector|VectorLength (- (Transformation|GetActorLocation) (Variables|Default|GetHook%20Location))) 5e+01)))
              (Variables|Default|SetNewCableLength _output_get)
              (Variables|/Script/CableComponent.CableComponent|SetEndLocation _cable "20.000000, 0,0.000000")))
          (else
            (bind _reached_location (CallFunction|MoveCable))
            (Variables|Default|SetHook%20Move%20Finished _reached_location)))))))

(event Collision|EventHit
  (params (MyComp :type Primitive%20Component%20Object%20Reference) (Other :type Actor%20Object%20Reference) (OtherComp :type Primitive%20Component%20Object%20Reference) (bSelfMoved :type Boolean) (HitLocation :type Vector :default "0, 0, 0") (HitNormal :type Vector :default "0, 0, 0") (NormalImpulse :type Vector :default "0, 0, 0") (Hit :type Hit%20Result%20Structure%20%28by%20ref%29))
  (Utilities|FlowControl|Sequence
    (:then_0
      ;[1 1 1] Damage + Knockback
      (if (== (Utilities|GetClass Other) "/Game/Blueprints/Bolt.Bolt_C")
        (bind _asbolt (Utilities|Casting|CastToBolt Other))
        (CallFunction|TakeDamage (Variables|/Game/Blueprints/Bolt.Bolt_C|GetDamage _asbolt))
        (Utilities|FlowControl|Sequence
          (:then_0
            ;[1 1 1] Blood Splatter screen
            (bind _asplayer_controller (Utilities|Casting|CastToPlayerController (Pawn|GetController)))
            (bind _returnvalue (UserInterface|CreateWidget "/Game/HUD/Blood_Splatter.Blood_Splatter_C" _asplayer_controller))
            (UserInterface|Viewport|AddtoPlayerScreen _returnvalue))
          (:then_1
            (Physics|AddForce (Variables|/Script/Engine.MovementComponent|GetUpdatedPrimitive (Variables|Character|GetCharacterMovement)) (* (Math|Vector|GetForwardVector (Variables|/Script/Engine.Actor|GetRootComponent Other)) 1.4e+04) "None" true)
            (Actor|DestroyActor Other))
          (:then_2
            (bind _asplayer_controller_2 (Utilities|Casting|CastToPlayerController (Pawn|GetController)))
            (Game|Feedback|PlayDynamicForceFeedback _asplayer_controller_2 0.3 0.3 true true true true))
          (:then_3
            (Variables|Default|SetLastHit (Variables|/Game/Blueprints/Bolt.Bolt_C|Getshooter _asbolt)) ; Set Last Hit
          ))))
    (:then_1
      ;[1 1 1] Die if touch outer sky (break out of level
      (if (== (Utilities|GetClass Other) "/Game/Blueprints/OuterSky.OuterSky_C")
        (CallFunction|BugFoundKillPlayer)))))

(event Input|ActionEvents|InputActionShootHarpoon
  (params (Key :type Key%20Structure))
  (bind _camera (Variables|Default|GetCamera))
  (bind _returnvalue (Transformation|GetWorldLocation _camera))
  ;[1 1 1] Harpoon/Change View
  ;;[1 1 1] Line trace
  (:Pressed
    (bind (_outhit _returnvalue_2) (Collision|LineTraceForObjects _returnvalue (+ _returnvalue (* (Math|Vector|GetForwardVector _camera) 4e+03)) (Utilities|Array|MakeArray "ObjectTypeQuery1" "ObjectTypeQuery2") false 0 "None"))
    (if _returnvalue_2
      ;;[1 1 1] Face Point and set hook
      (Transformation|SetActorRotation (Math|Rotator|MakeRotator 0.0 0.0 (.yaw (Math|Rotator|FindLookatRotation (Transformation|GetActorLocation) (.Location (Collision|BreakHitResult _outhit))))))
      (Utilities|FlowControl|Delay 0.6)
      (Variables|Default|SetHooked true)
      (Variables|Default|SetHook%20Location (.Location (Collision|BreakHitResult _outhit)))
      (else
        (CallFunction|StopGrapple)))))

(event Input|ActionEvents|InputActionChangeCameraView
  (params (Key :type Key%20Structure))
  (bind _camera (Variables|Default|GetCamera))
  (bind _first_person_camera (Variables|Default|GetFirst%20Person%20Camera))
  ;[1 1 1] Harpoon/Change View
  ;;[1 1 1] Change cameras
  (:Pressed
    (Utilities|FlowControl|FlipFlop
      (:A
        (Components|Activation|SetActive _camera false true)
        (Components|Activation|SetActive _first_person_camera true false))
      (:B
        (Components|Activation|SetActive _camera true false)
        (Components|Activation|SetActive _first_person_camera false true)))))

(event Input|ActionEvents|InputActionGrapple
  (params (Key :type Key%20Structure))
  ;[1 1 1] Harpoon/Change View
  (:Pressed
    (Variables|Default|SetGIsPressed true))
  (:Released
    (Variables|Default|SetGIsPressed false)))

(event Input|ActionEvents|InputActionMoveToDirection
  (params (Key :type Key%20Structure))
  ;[1 1 1] Player movement
  (:Pressed
    (bind _ispaused (CallFunction|IsGamePaused))
    (if (not _ispaused)
      (if (Variables|Default|GetCanPickDirection)
        (Variables|Default|SetMoving true)))))

(event Input|AxisEvents|InputAxisRotate
  (params (AxisValue :type Float%20%28single-precision%29))
  ;[1 1 1] Look around
  (bind _ispaused (CallFunction|IsGamePaused))
  (if (not _ispaused)
    (Transformation|AddLocalRotation (Variables|Collision|GetCapsuleComponent) (Math|Rotator|MakeRotator (* (Utilities|Time|GetWorldDeltaSeconds) AxisValue (Variables|Default|GetLook%20Speed)) 0.0 0.0) false false)))

(event Input|AxisEvents|InputAxisStartFire
  (params (AxisValue :type Float%20%28single-precision%29))
  ;[1 1 1] Fire
  (bind _ispaused (CallFunction|IsGamePaused))
  (if (not _ispaused)
    (if (== AxisValue 1.0)
      (bind _asbow_caster (Utilities|Casting|CastToBowCaster (Variables|/Script/Engine.ChildActorComponent|GetChildActor (Variables|Default|GetBowCaster))))
      (Default|FireBow _asbow_caster)
      (Physics|AddForce (Variables|/Script/Engine.MovementComponent|GetUpdatedPrimitive (Variables|Character|GetCharacterMovement)) (* (Math|Vector|GetForwardVector (Variables|Default|GetBowCaster)) -1e+01) "None" true))))

(event Input|AxisEvents|InputAxisTurn
  (params (AxisValue :type Float%20%28single-precision%29))
  ;[1 1 1] Look around
  (bind _ispaused (CallFunction|IsGamePaused))
  (if (not _ispaused)
    (Transformation|AddLocalRotation (Variables|Collision|GetCapsuleComponent) (Math|Rotator|MakeRotator 0.0 0.0 (* AxisValue (Utilities|Time|GetWorldDeltaSeconds) (Variables|Default|GetLook%20Speed))) false false)))

(event Input|AxisEvents|InputAxisLookup
  (params (AxisValue :type Float%20%28single-precision%29))
  ;[1 1 1] Look around
  (bind _ispaused (CallFunction|IsGamePaused))
  (if (not _ispaused)
    (Transformation|AddLocalRotation (Variables|Collision|GetCapsuleComponent) (Math|Rotator|MakeRotator 0.0 (* AxisValue (Utilities|Time|GetWorldDeltaSeconds) (Variables|Default|GetLook%20Speed)) 0.0) false false)))

(event Input|KeyboardEvents|K
  (params (Key :type Key%20Structure))
  ;[1 1 1] Temporary Kill Player
  (:Pressed
    (CallFunction|TakeDamage 99999999)))

(fn ConstructionScript
  (Transformation|AttachActorToActor (Components|GetOwner (Variables|Default|GetBowCaster)) (Components|GetOwner (Variables|Default|GetStaticMesh)) "None" "KeepRelative" "KeepRelative" "KeepRelative" true))

(fn MoveCable
  (bind _hook_location (Variables|Default|GetHook%20Location))
  (bind _cable (Variables|Default|GetCable))
  (bind _returnvalue (Transformation|GetWorldLocation _cable))
  (Rendering|SetVisibility _cable true false)
  (if (<= (Math|Vector|VectorLength (- _returnvalue _hook_location)) 1e+02)
    (return true)
    (else
      (Transformation|SetWorldLocation _cable (Math|Interpolation|VInterpTo _returnvalue _hook_location (Utilities|Time|GetWorldDeltaSeconds) 1e+01) false false)
      (return false))))

(fn IsGamePaused
  (bind _asbow_caster_game_mode (Utilities|Casting|CastToBowCasterGameMode (Game|GetGameMode)))
  (return (Variables|/Game/Blueprints/BowCasterGameMode.BowCasterGameMode_C|GettimerStopped _asbow_caster_game_mode)))