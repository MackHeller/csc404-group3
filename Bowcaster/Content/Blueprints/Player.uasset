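; Player character for a multiplayer bow-shooter, with class-based speed, damage or resistance and free look on pitch, yaw and roll.
; Movement is physics-driven: a force launches the player along the camera or toward a traced hook point until a capsule hit stops it.
; The child BowCaster fires with recoil, while incoming Bolts cause damage, knockback and last-hit tracking for the death screen.
; Tick aims the bow, draws a debug laser and runs a delayed idle-damage check.
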(event OnComponentHit(CapsuleComponent)
  (params (HitComponent :type Primitive%20Component%20Object%20Reference) (OtherActor :type Actor%20Object%20Reference) (OtherComp :type Primitive%20Component%20Object%20Reference) (NormalImpulse :type Vector :default "0, 0, 0") (Hit :type Hit%20Result%20Structure%20%28by%20ref%29))
  ;[1 1 1] Player movement
  (if (or (Variables|Default|GetMoving) (Variables|Default|GetGrappling))
    (Variables|Default|SetMoving false)
    (Variables|Default|SetGrappling false)
    (Variables|Default|SetCanPickDirection true)
    (CallFunction|StopMoving)
    (bind _asplayer_controller (Utilities|Casting|CastToPlayerController (Pawn|GetController)))
    (Game|Feedback|PlayDynamicForceFeedback _asplayer_controller 0.1 0.1 true true true true)))

(event Custom|SetClass
  (params (class-id :type Integer))
  (bind _defaultspeed (Variables|Default|GetDefaultSpeed))
  (bind _defaultdamage (Variables|Default|GetDefaultDamage))
  (bind _defaultresistance (Variables|Default|GetDefaultResistance))
  ;[1 1 1] Set Class
  (Development|PrintString (Utilities|String|ToString(Integer) class-id))
  (switch int class-id
    (:0
      (Variables|Default|SetSpeed-Class _defaultspeed)
      (Variables|Default|SetResistance-Class _defaultresistance)
      (Variables|Default|SetDamage-Class _defaultdamage))
    (:1
      (Variables|Default|SetSpeed-Class _defaultspeed)
      (Variables|Default|SetResistance-Class _defaultresistance)
      (Variables|Default|SetDamage-Class 55))
    (:2
      (Variables|Default|SetSpeed-Class 4.8e+04)
      (Variables|Default|SetResistance-Class _defaultresistance)
      (Variables|Default|SetDamage-Class _defaultdamage))
    (:3
      (Variables|Default|SetSpeed-Class _defaultspeed)
      (Variables|Default|SetResistance-Class 10)
      (Variables|Default|SetDamage-Class _defaultdamage))))

(event Custom|TakeDamage
  (params (damage :type Integer))
  (bind _resistance_class (Variables|Default|GetResistance-Class))
  ;[1 1 1] Taking Damage
  (if (> damage _resistance_class)
    (Variables|Default|SetHealth (- (Variables|Default|GetHealth) (- damage _resistance_class)))
    (else
      (Variables|Default|SetHealth (- (Variables|Default|GetHealth) damage))))
  (if (<= (Variables|Default|GetHealth) 0)
    (Variables|Default|SetHealth 0)
    (bind _asplayer_controller (Utilities|Casting|CastToPlayerController (Pawn|GetController)))
    (bind _returnvalue (UserInterface|CreateWidget "/Game/HUD/YouDied.YouDied_C" _asplayer_controller (Variables|Default|GetPlayerID) (Variables|Default|GetLastHit)))
    (UserInterface|Viewport|AddtoPlayerScreen _returnvalue)
    (Game|Feedback|PlayDynamicForceFeedback _asplayer_controller 1.0 1.0 true true true true)))

(event Custom|BugFoundKillPlayer
  ;[1 1 1] Bug Found, Show message and kill player
  (bind _asplayer_controller (Utilities|Casting|CastToPlayerController (Pawn|GetController)))
  (bind _returnvalue (UserInterface|CreateWidget "/Game/HUD/EasterEgg.EasterEgg_C" _asplayer_controller))
  (UserInterface|Viewport|AddtoPlayerScreen _returnvalue)
  (Utilities|FlowControl|Delay 3.5)
  (CallFunction|TakeDamage 99999999))

(event Custom|StopGrapple
  (bind _cable (Variables|Default|GetCable))
  ;[1 1 1] Hook
  ;;[1 1 1] Stop Grapple and reset cable length
  (Variables|Default|SetHooked false)
  (Transformation|SetWorldLocation (Variables|Default|GetCable) (Transformation|GetActorLocation) false false)
  (bind _output_get (Variables|/Script/CableComponent.CableComponent|SetCableLength _cable 0.0))
  (Variables|Default|SetNewCableLength _output_get)
  (Variables|/Script/CableComponent.CableComponent|SetEndLocation _cable "20.000000, 0,0.000000")
  (Variables|Default|SetHook%20Location "20.000000, 0, 0"))

(event Custom|StopMoving
  (bind _charactermovement (Variables|Character|GetCharacterMovement))
  (bind _updatedprimitive (Variables|/Script/Engine.MovementComponent|GetUpdatedPrimitive _charactermovement))
  ;[1 1 1] Player movement
  (Utilities|FlowControl|Sequence
    (:then_0
      (Class|PrimitiveComponent|SetAllPhysicsLinearVelocity _updatedprimitive "0, 0, 0" false)
      (Components|Movement|StopMovementImmediately (Variables|Character|GetCharacterMovement)))
    (:then_1
      (Class|PrimitiveComponent|SetAllPhysicsAngularVelocity _updatedprimitive (Math|Vector|RotateVector "0, 0, 0" "0, 0, 0") false)
      (Class|NavMovementComponent|StopActiveMovement (Variables|Character|GetCharacterMovement)))))

(event Custom|setBowRoation
  ;[1 1 1] Set Bow Rotation
  (Transformation|SetWorldRotation (Variables|Default|GetBowCaster) (|RoundRotation (Transformation|GetWorldRotation (Variables|Default|GetCamera))) false false))

(event Custom|GrappleWhenPressG
  ;[1 1 1] Hook
  ;;[1 1 1] Grapple when press G
  (CallFunction|GrapplingMove)
  (Variables|/Script/CableComponent.CableComponent|SetCableLength (Variables|Default|GetCable) (Math|Vector|VectorLength (- (Transformation|GetActorLocation) (Variables|Default|GetHook%20Location))))
  (CallFunction|StopGrapple))

(event Custom|Grappling%20Move
  ;[1 1 1] Hook
  ;;[1 1 1] Grappling Move
  (Variables|Default|SetGrappling true)
  (Utilities|FlowControl|Sequence
    (:then_0
      (Physics|AddForce (Variables|/Script/Engine.MovementComponent|GetUpdatedPrimitive (Variables|Character|GetCharacterMovement)) (* (- (Variables|Default|GetHook%20Location) (Transformation|GetActorLocation)) 3e+01) "None" true))
    (:then_1
      (Audio|SpawnSoundAttached "/Game/Art/Sound/SFX/15__Grappling_Hook_Wheeled_in.15__Grappling_Hook_Wheeled_in" (Variables|Default|GetCable)))))

(event EventBeginPlay
  (bind _cable (Variables|Default|GetCable))
  (Utilities|FlowControl|Sequence
    (:then_1
      ;[1 1 1] Spawn Player
      (Utilities|Casting|CastToBowCasterGameMode (Game|GetGameMode))
      (Variables|Default|SetSpawn%20Transform (Transformation|GetActorTransform)))
    (:then_2
      ;[1 1 1] Set cable parameters
      (Rendering|SetVisibility _cable false false)
      (Variables|/Script/CableComponent.CableComponent|SetCableLength _cable 0.0)
      (Variables|/Script/CableComponent.CableComponent|SetCableWidth _cable 2.0))
    (:then_3
      (Variables|Default|SetHealth 120))
    (:then_4
      (Components|Movement|StopMovementImmediately (Variables|Character|GetCharacterMovement)))
    (:then_5
      ;[1 1 1] SetOwnerOfBowCaster and set damage
      (bind _asbow_caster (Utilities|Casting|CastToBowCaster (Variables|/Script/Engine.ChildActorComponent|GetChildActor (Variables|Default|GetBowCaster))))
      (Variables|/Game/Blueprints/BowCaster.BowCaster_C|SetShooter _asbow_caster (Variables|Default|GetPlayerID))
      (Variables|/Game/Blueprints/BowCaster.BowCaster_C|SetDamage _asbow_caster (Variables|Default|GetDamage-Class)))))

(event EventTick
  (params (DeltaSeconds :type Float%20%28single-precision%29))
  (bind _bowcaster (Variables|Default|GetBowCaster))
  (bind _returnvalue (Transformation|GetWorldLocation _bowcaster))
  (Utilities|FlowControl|Sequence
    (:then_0
      (Utilities|FlowControl|Sequence
        (:then_0
          ;[1 1 1] Player movement
          (CallFunction|SetBowRoation)
          (if (and (Variables|Default|GetMoving) (Variables|Default|GetCanPickDirection))
            (Variables|Default|SetCanPickDirection false)
            (Physics|AddForce (Variables|/Script/Engine.MovementComponent|GetUpdatedPrimitive (Variables|Character|GetCharacterMovement)) (* (Math|Vector|GetForwardVector (Variables|Default|GetCamera)) (Variables|Default|GetSpeed-Class)) "None" true)))
        (:then_1
          ;[1 1 1] laser tracer
          (bind _outactors (Actor|GetAllActorsOfClass "/Game/Blueprints/Bolt.Bolt_C"))
          (Collision|LineTraceByChannel _returnvalue (+ (* (Math|Vector|GetForwardVector (Transformation|GetWorldRotation _bowcaster)) 1.5e+03) _returnvalue) "TraceTypeQuery3" false _outactors "ForOneFrame" true "(R=0.000000,G=1.000000,B=0.000000,A=1.000000)"))))
    (:then_1
      ;[1 1 1] Player takes damage if not moving
      (bind _ispaused (CallFunction|IsGamePaused))
      (if (not _ispaused)
        (Utilities|FlowControl|Delay 1.0)
        (if (Math|Vector|Equal(Vector) (Transformation|GetVelocity (stale _asplayer)) "0, 0, 0" 0.001)
          (CallFunction|TakeDamage 2)
          (Utilities|FlowControl|Sequence
            (:then_0
              (Utilities|FlowControl|Delay 3.0)
              (if (Math|Vector|Equal(Vector) (Transformation|GetVelocity) "0, 0, 0" 0.0001)
                (bind _returnvalue_2 (UserInterface|CreateWidget "/Game/Blueprints/NonMovingWarningMsg.NonMovingWarningMsg_C" (stale _asplayer_controller)))
                (UserInterface|Viewport|AddtoPlayerScreen _returnvalue_2)))
            (:then_1
              (bind _asplayer_controller (Utilities|Casting|CastToPlayerController (Pawn|GetController))))))))
    (:then_2
      ;[1 1 1] SetOwnerOfBowCaster and set damage
      (bind _asbow_caster (Utilities|Casting|CastToBowCaster (Variables|/Script/Engine.ChildActorComponent|GetChildActor (Variables|Default|GetBowCaster))))
      (Variables|/Game/Blueprints/BowCaster.BowCaster_C|SetShooter _asbow_caster (Variables|Default|GetPlayerID))
      (Variables|/Game/Blueprints/BowCaster.BowCaster_C|SetDamage _asbow_caster (Variables|Default|GetDamage-Class)))))

(event Collision|EventHit
  (params (MyComp :type Primitive%20Component%20Object%20Reference) (Other :type Actor%20Object%20Reference) (OtherComp :type Primitive%20Component%20Object%20Reference) (bSelfMoved :type Boolean) (HitLocation :type Vector :default "0, 0, 0") (HitNormal :type Vector :default "0, 0, 0") (NormalImpulse :type Vector :default "0, 0, 0") (Hit :type Hit%20Result%20Structure%20%28by%20ref%29))
  (Utilities|FlowControl|Sequence
    (:then_0
      ;[1 1 1] Damage + Knockback
      (if (== (Utilities|GetClass Other) "/Game/Blueprints/Bolt.Bolt_C")
        (bind _asbolt (Utilities|Casting|CastToBolt Other))
        (Variables|Default|SetLastHit (Variables|/Game/Blueprints/Bolt.Bolt_C|Getshooter _asbolt)) ; Set Last Hit
        (CallFunction|TakeDamage (Variables|/Game/Blueprints/Bolt.Bolt_C|GetDamage _asbolt))
        (Utilities|FlowControl|Sequence
          (:then_0
            ;[1 1 1] Blood Splatter screen
            (bind _asplayer_controller (Utilities|Casting|CastToPlayerController (Pawn|GetController)))
            (bind _returnvalue (UserInterface|CreateWidget "/Game/HUD/Blood_Splatter.Blood_Splatter_C" _asplayer_controller))
            (UserInterface|Viewport|AddtoPlayerScreen _returnvalue))
          (:then_1
            (Physics|AddForce (Variables|/Script/Engine.MovementComponent|GetUpdatedPrimitive (Variables|Character|GetCharacterMovement)) (* (Math|Vector|GetForwardVector (Variables|/Script/Engine.Actor|GetRootComponent Other)) 1.4e+04) "None" true)
            (Actor|DestroyActor Other))
          (:then_2
            (bind _asplayer_controller_2 (Utilities|Casting|CastToPlayerController (Pawn|GetController)))
            (Game|Feedback|PlayDynamicForceFeedback _asplayer_controller_2 0.3 0.3 true true true true)))))
    (:then_1
      ;[1 1 1] Die if touch outer sky (break out of level
      (if (== (Utilities|GetClass Other) "/Game/Blueprints/OuterSky.OuterSky_C")
        (CallFunction|BugFoundKillPlayer)))))

(event Input|ActionEvents|InputActionChangeCameraView
  (params (Key :type Key%20Structure))
  (bind _first_person_camera (Variables|Default|GetFirst%20Person%20Camera))
  (bind _camera (Variables|Default|GetCamera))
  ;[1 1 1] change camera view
  (:Pressed
    (Utilities|FlowControl|FlipFlop
      (:A
        (Components|Activation|SetActive _first_person_camera true false)
        (Components|Activation|SetActive _camera false false))
      (:B
        (Components|Activation|SetActive _camera true false)
        (Components|Activation|SetActive _first_person_camera false false)))))

(event Input|ActionEvents|InputActionShootHarpoon
  (params (Key :type Key%20Structure))
  (bind _first_person_camera (Variables|Default|GetFirst%20Person%20Camera))
  (bind _returnvalue (Transformation|GetWorldLocation _first_person_camera))
  ;[1 1 1] Hook
  ;;[1 1 1] Line trace
  (:Pressed
    (bind _ispaused (CallFunction|IsGamePaused))
    (if (not _ispaused)
      (bind _asbow_caster (Utilities|Casting|CastToBowCaster (Variables|/Script/Engine.ChildActorComponent|GetChildActor (Variables|Default|GetBowCaster))))
      (Default|ShootHook _asbow_caster)
      (bind (_outhit _returnvalue_2) (Collision|LineTraceForObjects _returnvalue (+ _returnvalue (* (Math|Vector|GetForwardVector _first_person_camera) 1e+04)) (Utilities|Array|MakeArray "ObjectTypeQuery1" "ObjectTypeQuery2") false 0 "None"))
      (if _returnvalue_2
        ;;[1 1 1] Face Point and set hook
        (Utilities|FlowControl|Delay 0.6)
        (Variables|Default|SetHooked true)
        (Variables|Default|SetHook%20Location (.Location (Collision|BreakHitResult _outhit)))
        (else
          (CallFunction|StopGrapple))))))

(event Input|ActionEvents|InputActionGrapple
  (params (Key :type Key%20Structure))
  (bind _cable (Variables|Default|GetCable))
  ;[1 1 1] Hook
  ;;[1 1 1] Pull
  (:Pressed
    (if (and (Variables|Default|GetHooked) (not (Variables|Default|GetGrappling)))
      (CallFunction|GrapplewhenPressG)
      (if (Variables|Default|GetHook%20Move%20Finished)
        (Utilities|FlowControl|Sequence
          (:then_0
            ;;[1 1 1] Move Start position of the cable
            (Transformation|SetWorldLocationAndRotation (Variables|Default|GetCable) (Math|Interpolation|VInterpTo (Transformation|GetWorldLocation (Variables|Default|GetCable)) (Variables|Default|GetHook%20Location) (Utilities|Time|GetWorldDeltaSeconds) 1e+02) (Math|Rotator|FindLookatRotation (Transformation|GetActorLocation) (Variables|Default|GetHook%20Location)) false false)
            ;;[1 1 1] Set cable length
            (bind _output_get (Variables|/Script/CableComponent.CableComponent|SetCableLength _cable (+ (Math|Vector|VectorLength (- (Transformation|GetActorLocation) (Variables|Default|GetHook%20Location))) 1e+01)))
            (Variables|Default|SetNewCableLength _output_get)
            (Variables|/Script/CableComponent.CableComponent|SetEndLocation _cable "20.000000, 0,0.000000")))))))

(event Input|ActionEvents|InputActionMoveToDirection
  (params (Key :type Key%20Structure))
  ;[1 1 1] Player movement
  (:Pressed
    (bind _ispaused (CallFunction|IsGamePaused))
    (if (not _ispaused)
      (if (Variables|Default|GetCanPickDirection)
        (Variables|Default|SetMoving true)))))

(event Input|AxisEvents|InputAxisRotate
  (params (AxisValue :type Float%20%28single-precision%29))
  ;[1 1 1] Look around
  (bind _ispaused (CallFunction|IsGamePaused))
  (if (not _ispaused)
    (Transformation|AddLocalRotation (Variables|Collision|GetCapsuleComponent) (Math|Rotator|MakeRotator (* (Utilities|Time|GetWorldDeltaSeconds) AxisValue (Variables|Default|GetLook%20Speed)) 0.0 0.0) false false)))

(event Input|AxisEvents|InputAxisTurn
  (params (AxisValue :type Float%20%28single-precision%29))
  ;[1 1 1] Look around
  (bind _ispaused (CallFunction|IsGamePaused))
  (if (not _ispaused)
    (Transformation|AddLocalRotation (Variables|Collision|GetCapsuleComponent) (Math|Rotator|MakeRotator 0.0 0.0 (* AxisValue (Utilities|Time|GetWorldDeltaSeconds) (Variables|Default|GetLook%20Speed))) false false)))

(event Input|AxisEvents|InputAxisLookup
  (params (AxisValue :type Float%20%28single-precision%29))
  ;[1 1 1] Look around
  (bind _ispaused (CallFunction|IsGamePaused))
  (if (not _ispaused)
    (Transformation|AddLocalRotation (Variables|Collision|GetCapsuleComponent) (Math|Rotator|MakeRotator 0.0 (* AxisValue (Utilities|Time|GetWorldDeltaSeconds) (Variables|Default|GetLook%20Speed)) 0.0) false false)))

(event Input|AxisEvents|InputAxisStartFire
  (params (AxisValue :type Float%20%28single-precision%29))
  ;[1 1 1] Fire
  (bind _ispaused (CallFunction|IsGamePaused))
  (if (not _ispaused)
    (if (== AxisValue 1.0)
      (bind _asbow_caster (Utilities|Casting|CastToBowCaster (Variables|/Script/Engine.ChildActorComponent|GetChildActor (Variables|Default|GetBowCaster))))
      (Default|FireBow _asbow_caster)
      (Physics|AddForce (Variables|/Script/Engine.MovementComponent|GetUpdatedPrimitive (Variables|Character|GetCharacterMovement)) (* (Math|Vector|GetForwardVector (Variables|Default|GetBowCaster)) -1e+01) "None" true))))

(event Input|KeyboardEvents|K
  (params (Key :type Key%20Structure))
  ;[1 1 1] Temporary Kill Player
  (:Pressed
    (CallFunction|TakeDamage 99999999)))

(fn ConstructionScript
  (Transformation|AttachActorToActor (Components|GetOwner (Variables|Default|GetBowCaster)) (Components|GetOwner (Variables|Default|GetStaticMesh)) "None" "KeepRelative" "KeepRelative" "KeepRelative" true))

(fn MoveCable
  (bind _hook_location (Variables|Default|GetHook%20Location))
  (bind _cable (Variables|Default|GetCable))
  (bind _returnvalue (Transformation|GetWorldLocation _cable))
  (Rendering|SetVisibility _cable true false)
  (if (<= (Math|Vector|VectorLength (- _returnvalue _hook_location)) 1e+02)
    (return true)
    (else
      (Transformation|SetWorldLocation _cable (Math|Interpolation|VInterpTo _returnvalue _hook_location (Utilities|Time|GetWorldDeltaSeconds) 1e+01) false false)
      (return false))))

(fn IsGamePaused
  (bind _asbow_caster_game_mode (Utilities|Casting|CastToBowCasterGameMode (Game|GetGameMode)))
  (return (Variables|/Game/Blueprints/BowCasterGameMode.BowCasterGameMode_C|GettimerStopped _asbow_caster_game_mode)))

(fn ChangeColour
  (params (ColourMaterial :type Material%20Object%20Reference))
  (Rendering|Material|SetMaterial (Variables|Default|GetCharacter_01) 0 ColourMaterial))