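; Forcefield actor that periodically adds child actors, apparently medpacks, at random points within its spawn area volumes.
; Tick gated by a 30-second Delay picks a point in the Medpack or Lower area bounds, though the random index 0–2 exceeds the two Select options.
; Each spawn plays an attached sound, and a 180-second Delay leads to component destruction.
; The Spawnmedpack function duplicates the spawn and sound without cleanup and is uncalled here.
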(event `self.ReceiveBeginPlay`)

(event `self.ReceiveTick`
  (params (DeltaSeconds :type "Float (single-precision)"))
  (bind (_origin _boxextent) (`KismetSystemLibrary.GetComponentBounds` (`self.medpackspawnarea`)))
  (bind (_origin_2 _boxextent_2) (`KismetSystemLibrary.GetComponentBounds` (`self.lowerspawnarea`)))
  (bind _x (.x _origin))
  (bind _y (.y _origin))
  (bind _z (.z _origin))
  (bind _x_2 (.x _boxextent))
  (bind _y_2 (.y _boxextent))
  (bind _z_2 (.z _boxextent))
  (bind _x_3 (.x _origin_2))
  (bind _y_3 (.y _origin_2))
  (bind _x_4 (.x _boxextent_2))
  (bind _y_4 (.y _boxextent_2))
  (`KismetSystemLibrary.Delay` 30.0)
  (bind _returnvalue (`AddComponent|NODE_AddChildActorComponent-2` :`RelativeTransform` (select `int` (`KismetMathLibrary.RandomIntegerInRange` 0 2) :`0` (`KismetMathLibrary.Conv_VectorToTransform` (`KismetMathLibrary.MakeVector` (`KismetMathLibrary.RandomFloatInRange` (- _x _x_2) (+ _x _x_2)) (`KismetMathLibrary.RandomFloatInRange` (- _y _y_2) (+ _y _y_2)) (`KismetMathLibrary.RandomFloatInRange` (- _z _z_2) (+ _z _z_2)))) :`1` (`KismetMathLibrary.Conv_VectorToTransform` (`KismetMathLibrary.MakeVector` (`KismetMathLibrary.RandomFloatInRange` (- _x_3 _x_4) (+ _x_3 _x_4)) (`KismetMathLibrary.RandomFloatInRange` (- _y_3 _y_4) (+ _y_3 _y_4)) (`KismetMathLibrary.RandomFloatInRange` (- (.z _origin_2) (.z _boxextent_2))))))))
  (`|ExecutionSequence`
    (:`then_0`
      (`KismetSystemLibrary.Delay` 180.0)
      (`ActorComponent.K2_DestroyComponent` _returnvalue))
    (:`then_1`
      (`GameplayStatics.SpawnSoundAttached` "/Game/Art/Sound/SFX/17__Medical_Pack_Spawn.17__Medical_Pack_Spawn" _returnvalue "None" (0.0 0.0 0.0) (struct) "KeepRelativeOffset" false 0.75))))

(fn `spawnmedpack`
  (bind (_origin _boxextent) (`KismetSystemLibrary.GetComponentBounds` (`self.medpackspawnarea`)))
  (bind (_origin_2 _boxextent_2) (`KismetSystemLibrary.GetComponentBounds` (`self.lowerspawnarea`)))
  (bind _x (.x _origin))
  (bind _y (.y _origin))
  (bind _z (.z _origin))
  (bind _x_2 (.x _boxextent))
  (bind _y_2 (.y _boxextent))
  (bind _z_2 (.z _boxextent))
  (bind _x_3 (.x _origin_2))
  (bind _y_3 (.y _origin_2))
  (bind _x_4 (.x _boxextent_2))
  (bind _y_4 (.y _boxextent_2))
  (bind _returnvalue (`AddComponent|NODE_AddChildActorComponent-1` :`RelativeTransform` (select `int` (`KismetMathLibrary.RandomIntegerInRange` 0 2) :`0` (`KismetMathLibrary.Conv_VectorToTransform` (`KismetMathLibrary.MakeVector` (`KismetMathLibrary.RandomFloatInRange` (- _x _x_2) (+ _x _x_2)) (`KismetMathLibrary.RandomFloatInRange` (- _y _y_2) (+ _y _y_2)) (`KismetMathLibrary.RandomFloatInRange` (- _z _z_2) (+ _z _z_2)))) :`1` (`KismetMathLibrary.Conv_VectorToTransform` (`KismetMathLibrary.MakeVector` (`KismetMathLibrary.RandomFloatInRange` (- _x_3 _x_4) (+ _x_3 _x_4)) (`KismetMathLibrary.RandomFloatInRange` (- _y_3 _y_4) (+ _y_3 _y_4)) (`KismetMathLibrary.RandomFloatInRange` (- (.z _origin_2) (.z _boxextent_2))))))))
  (`GameplayStatics.SpawnSoundAttached` "/Game/Art/Sound/SFX/17__Medical_Pack_Spawn.17__Medical_Pack_Spawn" _returnvalue "None" (0.0 0.0 0.0) (struct) "KeepRelativeOffset" false 0.75))

(fn `UserConstructionScript`)